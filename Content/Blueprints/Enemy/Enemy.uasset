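; Enemy actor that moves via projectile movement, with its initial speed set from a variable in the construction script.
; Overlapping a component tagged EndWall triggers EnemyCrash, which spawns a hit particle at the root and destroys the actor.
; WasHit calls AddScoreMessage on the player pawn to award a point, then runs the same crash.
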(event OnComponentBeginOverlap(Sphere)
  (params (OverlappedComponent :type Primitive%20Component%20Object%20Reference) (OtherActor :type Actor%20Object%20Reference) (OtherComp :type Primitive%20Component%20Object%20Reference) (OtherBodyIndex :type Integer) (bFromSweep :type Boolean) (SweepResult :type Hit%20Result%20Structure%20%28by%20ref%29))
  (if (Components|ComponentHasTag OtherComp "EndWall")
    (CallFunction|EnemyCrash)))

(event EventWasHit
  (Class|BPIPlayer|AddScore(Message) (Game|Player|GetPlayerPawn 0) 1)
  (CallFunction|EnemyCrash))

(fn ConstructionScript
  (Variables|/Script/Engine.ProjectileMovementComponent|SetInitialSpeed (Variables|Default|GetProjectileMovement) (Variables|Default|GetInitialSpeed)))

(fn EnemyCrash
  (Effects|SpawnEmitteratLocation "/Game/Particles/HitEnemyParticle.HitEnemyParticle" (Transformation|GetWorldLocation (Variables|Default|GetRoot self)))
  (Actor|DestroyActor))