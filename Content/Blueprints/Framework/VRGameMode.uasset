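; VR game mode that runs a wave-based enemy game, with start, reset and quit events.
; It caches all EnemySpawner actors and the in-game menu, which it hides on start and shows again on reset.
; Each wave shuffles the spawners, triggers as many as EnemiesPerWave specifies, then schedules the next wave with a timer, resetting the game once the wave list runs out.
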(event Custom|Start%20Game
  (bind _menuactor (Variables|Default|GetMenuActor))
  (if (not (Variables|Default|GetGameRuning?))
    (CallFunction|SpawnEnemyWave)
    (Variables|Default|SetGameRuning? true)
    (Rendering|SetActorHiddenInGame _menuactor true)
    (Collision|SetActorEnableCollision _menuactor false)
    (Class|BPIPlayer|ResetScore(Message) (Game|Player|GetPlayerPawn 0))))

(event Custom|Quit%20Game
  (Game|QuitGame 0 "Quit"))

(event Custom|Reset%20Game
  (bind _menuactor (Variables|Default|GetMenuActor))
  (Variables|Default|SetGameRuning? false)
  (Rendering|SetActorHiddenInGame _menuactor false)
  (Collision|SetActorEnableCollision _menuactor true)
  (Variables|Default|SetWaveIndex 0))

(event EventBeginPlay
  (bind _outactors (Actor|GetAllActorsOfClass "/Game/Blueprints/Enemy/EnemySpawner.EnemySpawner_C"))
  (Variables|Default|SetEnemySpawners _outactors)
  (bind _outactors_2 (Actor|GetAllActorsOfClass "/Game/Blueprints/HUD/BP_InGameMenu.BP_InGameMenu_C"))
  (Variables|Default|SetMenuActor (Utilities|Array|Get(acopy) _outactors_2)))

(fn ConstructionScript)

(fn SpawnEnemyWave
  (if (> (Variables|Default|GetWaveIndex) (Utilities|Array|LastIndex (Variables|Default|GetEnemiesPerWave)))
    (CallFunction|ResetGame)
    (else
      (Utilities|Array|Shuffle (Variables|Default|GetEnemySpawners))
      (for _index (range 0 (- (Utilities|Array|Get(acopy) (Variables|Default|GetEnemiesPerWave) (Variables|Default|GetWaveIndex)) 1))
        (Default|HandleEnemySpawn (Utilities|Array|Get(acopy) (Variables|Default|GetEnemySpawners) _index)))
      (Utilities|Time|SetTimerbyFunctionName 0 "SpawnEnemyWave" (Variables|Default|GetDelayPerWave))
      (Math|Integer|IncrementInt (Variables|Default|GetWaveIndex)))))